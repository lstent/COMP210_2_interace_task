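; A countdown timer Blueprint that shows the remaining whole seconds on a text render component.
; Each tick it subtracts delta time from a float counter and writes the truncated value to the text.
; While the counter is below zero it calls TimerEnd on VRGameMode every tick, as nothing here stops or resets it.
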(event `self.ReceiveTick`
  (params (DeltaSeconds :type "Float (single-precision)"))
  (bind _output_get (set `self.floatTime` (- (`self.floatTime`) DeltaSeconds)))
  (bind _output_get_2 (set `self.integerTime` (`KismetMathLibrary.FTrunc` _output_get)))
  (`TextRenderComponent.K2_SetText` (`self.TextRender`) (`KismetTextLibrary.Conv_IntToText` _output_get_2))
  (if (< (`self.floatTime`) 0.0)
    (bind _asvrgame_mode (cast `/Game/Blueprints/GameMode/VRGameMode` (`GameplayStatics.GetGameMode`)))
    (`/Game/Blueprints/GameMode/VRGameMode.timerEnd` _asvrgame_mode)))

(fn `UserConstructionScript`)