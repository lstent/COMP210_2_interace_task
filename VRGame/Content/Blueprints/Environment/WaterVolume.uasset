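; Water volume Blueprint that tracks whether the Great White and several other actor types are inside its box.
; Overlap events run a chain of casts, with only the GreatWhite class resolved, to update each actor's IsInWater flag.
; Entering sets the flag true, except in the fourth branch, which sets it false.
; Leaving clears the flag and deactivates the actor's Bubbles effect; entering does not reactivate it.
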(event `self.Box.OnComponentBeginOverlap`
  (params (OverlappedComponent :type "PrimitiveComponent Object Reference") (OtherActor :type "Actor Object Reference") (OtherComp :type "PrimitiveComponent Object Reference") (OtherBodyIndex :type Integer) (bFromSweep :type Boolean) (SweepResult :type "HitResult Structure (by ref)"))
  ;[1 1 1] particle effects will play in water after it overlaps again.
  (bind _asgreat_white (cast `/Game/Blueprints/Player/GreatWhite/GreatWhite` OtherActor)
    (:`then`
      (set `/Game/Blueprints/Player/GreatWhite/GreatWhite.IsInWater` true _asgreat_white))
    (:`CastFailed`
      (bind _asthresher (cast `` OtherActor)
        (:`then`
          (set `/Game/Blueprints/Environment/WaterVolume.IsInWater` true _asthresher))
        (:`CastFailed`
          (bind _asmako (cast `` OtherActor)
            (:`then`
              (set `/Game/Blueprints/Environment/WaterVolume.IsInWater` true _asmako))
            (:`CastFailed`
              (bind _asnurse (cast `` OtherActor)
                (:`then`
                  (set `/Game/Blueprints/Environment/WaterVolume.IsInWater` false _asnurse))
                (:`CastFailed`
                  (bind _asbp_hammerhead (cast `` OtherActor)
                    (:`then`
                      (set `/Game/Blueprints/Environment/WaterVolume.IsInWater` true _asbp_hammerhead))
                    (:`CastFailed`
                      (bind _aswhale (cast `` OtherActor))
                      (set `/Game/Blueprints/Environment/WaterVolume.IsInWater` true _aswhale))))))))))))

(event `self.Box.OnComponentEndOverlap`
  (params (OverlappedComponent :type "PrimitiveComponent Object Reference") (OtherActor :type "Actor Object Reference") (OtherComp :type "PrimitiveComponent Object Reference") (OtherBodyIndex :type Integer))
  ;[1 1 1] particle effect stops outside water and wont play when used outside water
  (bind _asgreat_white (cast `/Game/Blueprints/Player/GreatWhite/GreatWhite` OtherActor)
    (:`then`
      (set `/Game/Blueprints/Player/GreatWhite/GreatWhite.IsInWater` false _asgreat_white)
      (`ActorComponent.Deactivate` (`/Game/Blueprints/Player/GreatWhite/GreatWhite.Bubbles` _asgreat_white)))
    (:`CastFailed`
      (bind _asthresher (cast `` OtherActor)
        (:`then`
          (set `/Game/Blueprints/Environment/WaterVolume.IsInWater` false _asthresher)
          (`ActorComponent.Deactivate` (`/Game/Blueprints/Environment/WaterVolume.Bubbles` _asthresher)))
        (:`CastFailed`
          (bind _asmako (cast `` OtherActor)
            (:`then`
              (set `/Game/Blueprints/Environment/WaterVolume.IsInWater` false _asmako)
              (`ActorComponent.Deactivate` (`/Game/Blueprints/Environment/WaterVolume.Bubbles` _asmako)))
            (:`CastFailed`
              (bind _asnurse (cast `` OtherActor)
                (:`then`
                  (set `/Game/Blueprints/Environment/WaterVolume.IsInWater` false _asnurse)
                  (`ActorComponent.Deactivate` (`/Game/Blueprints/Environment/WaterVolume.Bubbles` _asnurse)))
                (:`CastFailed`
                  (bind _asbp_hammerhead (cast `` OtherActor)
                    (:`then`
                      (set `/Game/Blueprints/Environment/WaterVolume.IsInWater` false _asbp_hammerhead)
                      (`ActorComponent.Deactivate` (`/Game/Blueprints/Environment/WaterVolume.Bubbles` _asbp_hammerhead)))
                    (:`CastFailed`
                      (bind _aswhale (cast `` OtherActor))
                      (set `/Game/Blueprints/Environment/WaterVolume.IsInWater` false _aswhale)
                      (`ActorComponent.Deactivate` (`/Game/Blueprints/Environment/WaterVolume.Bubbles` _aswhale)))))))))))))

(fn `UserConstructionScript`)