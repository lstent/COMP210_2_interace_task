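; VRGameMode is a game mode that handles the win and lose screens for a game tracked by a Fish count.
; Its timerEnd event shows the Loser widget, gives UI-only input focus to its Again button and pauses the game.
; Tick prints Fish every frame and, while it equals zero, repeatedly creates a Winner widget with the same focus setup but without pausing.
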(event `timerEnd`
  (bind _returnvalue (`|CreateWidget` "/Game/Blueprints/UI/loser.loser_C"))
  (`UserWidget.AddToViewport` _returnvalue 0)
  (`WidgetBlueprintLibrary.SetInputMode_UIOnlyEx` (`GameplayStatics.GetPlayerController` 0) (`/Game/Blueprints/UI/loser.Again` _returnvalue))
  (`GameplayStatics.SetGamePaused` true))

(event `self.ReceiveTick`
  (params (DeltaSeconds :type "Float (single-precision)"))
  (`KismetSystemLibrary.PrintString` (`KismetStringLibrary.Conv_IntToString` (`self.fish`)))
  (if (== (`self.fish`) 0)
    (bind _returnvalue (`|CreateWidget` "/Game/Blueprints/UI/Winner.Winner_C"))
    (`UserWidget.AddToViewport` _returnvalue 0)
    (`WidgetBlueprintLibrary.SetInputMode_UIOnlyEx` (`GameplayStatics.GetPlayerController` 0) (`/Game/Blueprints/UI/Winner.Again` _returnvalue))))

(fn `UserConstructionScript`)