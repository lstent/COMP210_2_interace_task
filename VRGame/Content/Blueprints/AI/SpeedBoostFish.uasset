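; Swimming AI fish pickup that registers itself in the VRGameMode fish count on BeginPlay.
; Tick issues AIMoveTo toward random navigable points, using an Ismoving flag and random delay, and nudges the fish upward when a move fails.
; Capsule hits from the MotionControllerPawn spawn a pickup particle, play controller force feedback, decrement the count and destroy the fish.
; Despite the name, it grants no speed boost to the player.
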(event `self.ReceiveBeginPlay`
  ;[1 1 1] Add 1 to total fish in beginning of level
  (bind _asvrgame_mode (cast `/Game/Blueprints/GameMode/VRGameMode` (`GameplayStatics.GetGameMode`)))
  (set `/Game/Blueprints/GameMode/VRGameMode.fish` (+ (`/Game/Blueprints/GameMode/VRGameMode.fish` _asvrgame_mode) 1) _asvrgame_mode))

(event `self.ReceiveTick`
  (params (DeltaSeconds :type "Float (single-precision)"))
  ;[1 1 1] MoveTo
  (if (not (`self.Ismoving`))
    (`|AIMoveTo` self (`NavigationSystem.K2_GetRandomLocationInNavigableRadius` (`SceneComponent.K2_GetComponentLocation` (`self.Mesh`)) 10000.0)
      (:`then`
        (set `self.Ismoving` true :!label _label)
        (set `CharacterMovementComponent.MaxSwimSpeed` 1000.0 (`self.CharacterMovement`))
        (`KismetSystemLibrary.Delay` (`KismetMathLibrary.RandomFloatInRange` 1.0 10.0)))
      (:`OnSuccess`
        (goto _label))
      (:`OnFail`
        (`self.K2_SetActorLocation` self (+ (`SceneComponent.K2_GetComponentLocation` (`self.Mesh`)) (0.0 0.0 10.0)) false false)))
    (set `self.Ismoving` false)))

(event `self.CapsuleComponent.OnComponentHit`
  (params (HitComponent :type "PrimitiveComponent Object Reference") (OtherActor :type "Actor Object Reference") (OtherComp :type "PrimitiveComponent Object Reference") (NormalImpulse :type "Vector Structure") (Hit :type "HitResult Structure (by ref)"))
  ;[1 1 1] Fish death and minus 1 from total fish in level
  (cast `/Game/VirtualRealityBP/Blueprints/MotionControllerPawn` OtherActor)
  (`GameplayStatics.SpawnEmitterAtLocation` "/Game/Particles/PickUp/P_pickup.P_pickup" (`self.K2_GetActorLocation`))
  (`PlayerController.PlayDynamicForceFeedback` (`GameplayStatics.GetPlayerController` 0) 0.3 0.5 true true true true)
  (bind _asvrgame_mode (cast `/Game/Blueprints/GameMode/VRGameMode` (`GameplayStatics.GetGameMode`)))
  (set `/Game/Blueprints/GameMode/VRGameMode.fish` (- (`/Game/Blueprints/GameMode/VRGameMode.fish` _asvrgame_mode) 1) _asvrgame_mode)
  (`self.K2_DestroyActor`))

(fn `UserConstructionScript`)